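; Base actor for pickup items in the item system, carrying an ItemInfo struct that describes the item.
; Its construction script rebuilds ItemInfo, keeping type, name, image and index while setting the actor's own class and fixed values for the remaining fields.
; When interacted with, it checks the instigator for inventory space, passes ItemInfo through PickUpMessage and destroys itself.
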(event `/Game/ItemSystem/ItemIterFace_BP.Interactable`
  (params (Instigator :type "/Game/Charcter/Player/Player Object Reference"))
  ;[1 1 1] アイテム拾ったら消す
  (if (`/Game/Charcter/Player/Player.HasSpaceInventroy` Instigator)
    (message `/Game/ItemSystem/ItemIterFace_BP.PickUp` Instigator (`self.ItemInfo`))
    (`self.K2_DestroyActor`)))

(fn `UserConstructionScript`
  (bind (_iteminfo_itemtype _iteminfo_itemname _iteminfo_itemclass _iteminfo_itemimage _iteminfo_itemindex) (break `/Game/ItemSystem/ItemInfo` (`self.ItemInfo`)))
  (`parent.UserConstructionScript`)
  ;[1 1 1] アイテムDataを代入する
  (set `self.ItemInfo` (make `/Game/ItemSystem/ItemInfo` _iteminfo_itemtype _iteminfo_itemname (`GameplayStatics.GetObjectClass` self) _iteminfo_itemimage _iteminfo_itemindex)))