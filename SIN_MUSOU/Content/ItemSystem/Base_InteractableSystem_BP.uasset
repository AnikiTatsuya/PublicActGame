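; Base interactable item Blueprint that the player can detect by proximity and highlight.
; ItemArea overlaps register and unregister the item with the overlapping Player as an interactable.
; SetHighLight swaps placeholder TextRender text and toggles both custom depth and main-pass rendering on ItemMesh and ItemArea.
; The highlight is provisional, as no highlight material exists yet.
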(event `self.ItemArea.OnComponentBeginOverlap`
  (params (OverlappedComponent :type "PrimitiveComponent Object Reference") (OtherActor :type "Actor Object Reference") (OtherComp :type "PrimitiveComponent Object Reference") (OtherBodyIndex :type Integer) (bFromSweep :type Boolean) (SweepResult :type "HitResult Structure (by ref)"))
  (bind _asplayer (cast `/Game/Charcter/Player/Player` OtherActor))
  (message `/Game/ItemSystem/ItemIterFace_BP.RegisterInteractable` _asplayer self))

(event `self.ItemArea.OnComponentEndOverlap`
  (params (OverlappedComponent :type "PrimitiveComponent Object Reference") (OtherActor :type "Actor Object Reference") (OtherComp :type "PrimitiveComponent Object Reference") (OtherBodyIndex :type Integer))
  (bind _asplayer (cast `/Game/Charcter/Player/Player` OtherActor))
  (message `/Game/ItemSystem/ItemIterFace_BP.UnregisterInteractable` _asplayer self))

(fn `SetHighLight`
  (params (IsHighLight :type Boolean))
  (bind _textrender (`self.TextRender`))
  (if IsHighLight
    (`TextRenderComponent.K2_SetText` _textrender (`KismetTextLibrary.Conv_StringToText` "Yessssss!"))
    (else
      (`TextRenderComponent.K2_SetText` _textrender (`KismetTextLibrary.Conv_StringToText` "Nooooooooo!"))))
  ;[1 1 1] ハイライトマテリアルがないため一旦ここまで
  (`PrimitiveComponent.SetRenderCustomDepth` (`self.ItemMesh`) IsHighLight)
  (`PrimitiveComponent.SetRenderCustomDepth` (`self.ItemArea`) IsHighLight)
  (`PrimitiveComponent.SetRenderInMainPass` (`self.ItemArea`) IsHighLight)
  (`PrimitiveComponent.SetRenderInMainPass` (`self.ItemMesh`) IsHighLight))

(fn `UserConstructionScript`)